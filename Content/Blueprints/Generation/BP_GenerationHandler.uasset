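; BP_GenerationHandler spawns a grid of BP_Chunk tiles when play begins.
; It first spawns a temporary chunk with the smallest mesh, reads its landscape mesh bounds to get the tile size, then destroys it.
; Nested row and column loops then place chunks spaced by tile size plus GridSpacing, passing each its row and column.
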(event EventBeginPlay
  (CallFunction|GenerateGrid))

(fn ConstructionScript)

(fn GenerateGrid
  (bind _gridspacing (Variables|GridSetup|GetGridSpacing))
  (CallFunction|CalculateTileSize)
  (for _index (range 0 (- (Variables|GridSetup|GetGridRows) 1))
    (Variables|GridSetup|SetCurrentRow _index)
    (for _index_2 (range 0 (- (Variables|GridSetup|GetGridColumns) 1))
      (Variables|GridSetup|SetCurrentColumn _index_2)
      (Game|SpawnActorfromClass "/Game/Blueprints/Generation/BP_Chunk.BP_Chunk_C" (Math|Transform|MakeTransform (Math|Vector|MakeVector (+ (* (Variables|GridSetup|GetCurrentRow) _gridspacing) (* (Variables|GridSetup|GetCurrentRow) (Variables|Default|GetTileSize))) (+ (* _gridspacing (Variables|GridSetup|GetCurrentColumn)) (* (Variables|GridSetup|GetCurrentColumn) (Variables|Default|GetTileSize))) 0.0) "0, 0, 0" "1.000000,1.000000,1.000000") "Undefined" 0 (Variables|GridSetup|GetCurrentColumn) (Variables|GridSetup|GetCurrentRow) true 0))))

(fn CalculateTileSize
  (bind _returnvalue (Game|SpawnActorfromClass "/Game/Blueprints/Generation/BP_Chunk.BP_Chunk_C" (Math|Transform|MakeTransform "0, 0, 0" "0, 0, 0" "1.000000,1.000000,1.000000") "Undefined" 0 0 0 true 0))
  (Variables|Default|SetTileSize (* (.x (.BoxExtent (Collision|GetComponentBounds (Variables|/Game/Blueprints/Generation/BP_Chunk.BP_Chunk_C|GetLandscapeMesh _returnvalue)))) 2.0))
  (Actor|DestroyActor _returnvalue))