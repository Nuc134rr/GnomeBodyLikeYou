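; BP_Chunk is a world-generation chunk that picks a landscape mesh and scatters toadstools on it.
; The construction script sets a random or fixed smallest mesh, then spawns a random number of toadstool components attached to it.
; Each retries swept relative transforms from RandomTransformWithinMeshBounds until no blocking hit is reported.
; That helper's random location, yaw and scale logic appears unconnected.
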(fn ConstructionScript
  (bind _landscapemesh (Variables|Default|GetLandscapeMesh))
  (Utilities|FlowControl|Sequence
    (:then_0
      (if (Variables|Default|GetUseSmallestMesh)
        (Components|StaticMesh|SetStaticMesh _landscapemesh "/Game/Meshes/ProgrammerArt/SM_GeorgeProArt.SM_GeorgeProArt")
        (else
          (Components|StaticMesh|SetStaticMesh _landscapemesh (.OutItem (Utilities|Array|Random (LocalVariables|GetLandscapeMeshes)))))))
    (:then_2
      (CallFunction|CreateEnvironmentMeshes "/Game/Meshes/SM_Toadstool.SM_Toadstool" (Variables|Default|GetMaxMushroomSpawns)))))

(fn CreateEnvironmentMeshes
  (params (Mesh :type Static%20Mesh%20Object%20Reference) (Instances :type Integer))
  (for _index (range 0 (Math|Random|RandomIntegerinRange 0 (- Instances 1)))
    (bind _returnvalue (AddComponent|AddStaticMeshComponent true))
    (bind _output_get (LocalVariables|SetCurrentMesh _returnvalue))
    (Components|StaticMesh|SetStaticMesh _output_get Mesh)
    (Transformation|AttachComponentToComponent (LocalVariables|GetCurrentMesh) (Variables|Default|GetLandscapeMesh) "None" "KeepRelative" "KeepRelative" "KeepRelative" true)
    (while (LocalVariables|GetHitResult)
      (bind _sweephitresult (Transformation|SetRelativeTransform (LocalVariables|GetCurrentMesh) (Utilities|RandomTransformWithinMeshBounds (Variables|Default|GetLandscapeMesh)) true true))
      (bind _output_get_2 (LocalVariables|SetHitResult (.bblockinghit _sweephitresult)))
      (if _output_get_2
        (LocalVariables|SetHitAtLeastOnce true)))
    (LocalVariables|SetHitResult true)
    (if (LocalVariables|GetHitAtLeastOnce)
      (Development|PrintString "Successfully moved" true true "(R=0.997405,G=0.099455,B=1.000000,A=1.000000)"))))