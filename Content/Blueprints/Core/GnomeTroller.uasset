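; GnomeTroller is a player controller that toggles between character control and mouse-driven UI.
; Bound start and stop mouse events either unpossess the pawn, show the cursor and lock input to UI only, or repossess player character 0 and hide the cursor.
; Stopping does not reset the input mode.
; Tick prints the selected slot's display name as debug text.
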(event Custom|StartMouseInput
  (Pawn|UnPossess)
  (Variables|Default|SetbShowMouseCursor true)
  (Variables|Default|SetbEnableClickEvents true)
  (Input|SetInputModeUIOnly 0 0 "LockAlways" false))

(event Custom|StopMouseInput
  (Pawn|Possess (Game|GetPlayerCharacter 0))
  (Variables|Default|SetbShowMouseCursor false)
  (Variables|Default|SetbEnableClickEvents false))

(event EventTick
  (params (DeltaSeconds :type Float%20%28single-precision%29))
  (Development|PrintString (Utilities|String|ToString(Text) (.displayname (Variables|Default|GetSelectedSlotData))) true true "(R=0.000000,G=0.660000,B=1.000000,A=1.000000)" DeltaSeconds))

(event EventBeginPlay
  (EventDispatchers|BindEventtoStartMouse (delegate Custom|StartMouseInput))
  (EventDispatchers|BindEventtoEndMouse (delegate Custom|StopMouseInput)))

(fn ConstructionScript)