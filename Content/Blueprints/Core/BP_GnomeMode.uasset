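; Game mode for a mushroom-foraging round in which the player builds a bouquet for a randomly chosen gnome.
; BeginPlay loads that gnome's bio, sprites and mushroom preferences from a data table, then starts the foraging timer, which Tick reads as a countdown.
; When time expires, it hides the gameplay HUD and opens the bouquet widget with UI-only input.
; BouquetDecision scores the bouquet by summing each mushroom's count times its points for that gnome.
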(event Custom|BaddieDecision
  (bind _outrownames (DataTable|GetDataTableRowNames "/Game/Blueprints/Core/Gnome_Love_Mushroom_doc_-_Sheet1.Gnome_Love_Mushroom_doc_-_Sheet1"))
  (bind _output_get (Variables|Gnome|SetCurrentGnome (.OutItem (Utilities|Array|Random _outrownames))))
  (bind _returnvalue (Utilities|GetDataTableRow "/Game/Blueprints/Core/Gnome_Love_Mushroom_doc_-_Sheet1.Gnome_Love_Mushroom_doc_-_Sheet1" _output_get)
    (:then
      (Variables|Gnome|SetMushroomPoints (.mushroompoints _returnvalue))
      (Variables|Gnome|SetCurrentGnomeBio (Utilities|Array|MakeArray (.bio1 _returnvalue) (.bio2 _returnvalue) (.bio3 _returnvalue)))
      (Variables|Gnome|SetGnomeMushyThumbnail (.mushythumbnails _returnvalue))
      (Variables|Gnome|SetGnomeSprites (.gnomesprites _returnvalue))
      (Variables|Gnome|SetGnomeName (.name _returnvalue)))))

(event Custom|BouquetDecision
  (params (MushroomBouquet :type Map%20of%20Names%20to%20Integers))
  (bind _output_get (Variables|MushroomBouquet|SetMushroomBouquet MushroomBouquet))
  (bind _keys (Utilities|Map|Keys _output_get))
  (Variables|MushroomBouquet|SetMushroomBouquetNames _keys)
  (bind _values (Utilities|Map|Values (Variables|MushroomBouquet|GetMushroomBouquet)))
  (Variables|MushroomBouquet|SetMushroomPointsMultiplier _values)
  (for _array_element (Variables|MushroomBouquet|GetMushroomBouquetNames)
    (Variables|MushroomBouquet|SetCurrentPoints (+ (Variables|MushroomBouquet|GetCurrentPoints) (* (.Value (Utilities|Map|Find (Variables|MushroomBouquet|GetMushroomBouquet) _array_element)) (.Value (Utilities|Map|Find (Variables|Gnome|GetMushroomPoints) _array_element)))))))

(event Custom|StartForagingTime
  (CallFunction|SpawnHUD)
  (bind _returnvalue (Utilities|Time|SetTimerbyFunctionName 0 "TimerWidget" (Variables|Foraging|GetForagingTime)))
  (Variables|Default|SetTimerHandle _returnvalue)
  (Utilities|FlowControl|Delay (Variables|Foraging|GetForagingTime))
  (CallFunction|BouquetMaker))

(event Custom|BouquetMaker
  (bind _returnvalue (Game|GetPlayerController 0))
  (bind _asgnome_troller (Utilities|Casting|CastToGnomeTroller _returnvalue))
  (Widget|SetVisibility (Variables|/Game/Blueprints/Widgets/GameplayHUD.GameplayHUD_C|GetHUD (.AsGameplay%20HUD (Utilities|Casting|CastToGameplayHUD (HUD|GetHUD (Game|GetPlayerController 0))))) "Hidden")
  (bind _returnvalue_2 (UserInterface|CreateWidget "/Game/Blueprints/Widgets/BouquetMaker/WBP_BouquetHUD.WBP_BouquetHUD_C"))
  (bind _output_get (Variables|Widgets|SetBouquetHUD _returnvalue_2))
  (UserInterface|Viewport|AddtoViewport _output_get 0)
  (Variables|/Script/Engine.PlayerController|SetbShowMouseCursor _asgnome_troller true)
  (Input|SetInputModeUIOnly _asgnome_troller (Variables|Widgets|GetBouquetHUD) "LockAlways" false))

(event Custom|SpawnHUD)

(event EventBeginPlay
  (CallFunction|BaddieDecision)
  (CallFunction|StartForagingTime))

(event EventTick
  (params (DeltaSeconds :type Float%20%28single-precision%29))
  (Variables|Default|SetTimerRemaining (Math|Float|Floor (Utilities|Time|GetTimerRemainingTimebyHandle (Variables|Default|GetTimerHandle)))))

(fn ConstructionScript)

(fn TimerWidget)