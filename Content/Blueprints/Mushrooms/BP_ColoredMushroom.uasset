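; Colored mushroom actor that seeds a cluster of copies of itself and snaps to the ground.
; Construction randomly picks a color index and, for non-spawned mushrooms, a mesh.
; On BeginPlay, a non-spawned mushroom scatters flagged copies within a temporary box, shares its mesh, and sets its own ItemID from the color's data table row.
; Every mushroom then line traces downward, with persistent debug drawing, and moves to the hit.
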(event EventBeginPlay
  (Utilities|FlowControl|Sequence
    (:then_0
      (if (not (Variables|Default|GetbSpawnedFromMushroom))
        (bind _returnvalue (AddComponent|AddBoxComponent false (Math|Transform|MakeTransform "0, 0, 0" "0, 0, 0" "3.000000,3.000000,0.100000")))
        (for _index (range 0 (Variables|Default|GetMushroomGroupSize))
          (bind _returnvalue_2 (Game|SpawnActorfromClass "BP_ColoredMushroom_C" (Math|Transform|MakeTransform (+ (.location (Utilities|RandomTransformWithinComponentBounds _returnvalue)) (Transformation|GetWorldLocation (Variables|Default|GetMeshroom))) (.rotation (Utilities|RandomTransformWithinComponentBounds _returnvalue)) (.scale (Utilities|RandomTransformWithinComponentBounds _returnvalue))) "Undefined" 0 true 0))
          (Components|StaticMesh|SetStaticMesh (Variables|/Game/Blueprints/Core/BP_BaseCollectableMushroom.BP_BaseCollectableMushroom_C|GetMeshroom _returnvalue_2) (Variables|/Script/Engine.StaticMeshComponent|GetStaticMesh (Variables|Default|GetMeshroom)))
          (bind _returnvalue_3 (Utilities|GetDataTableRow "/Game/Blueprints/Core/Inventory/ItemDataTable.ItemDataTable" (Utilities|String|StringToName (Utilities|String|Append (Utilities|Select :Index (Variables|Default|GetMeshroomIndex) :Option%200 "Red" :Option%201 "Yellow" :Option%202 "Green" :Option%203 "Blue" :Option%204 "Purple" :Option%205 "Pink" :Option%206 "Brown" :Option%207 "White" :Option%208 "Black" :Option%209 "Flatcap" :Option%2010 "Poison" :Option%2011 "Prismatic") "Mushroom")))
            (:then
              (Variables|/Game/Blueprints/Core/Inventory/ItemDataComponent.ItemDataComponent_C|SetItemID (Variables|Default|GetItemDataComponent) _returnvalue_3))))))
    (:then_1
      (bind _outhit (Collision|LineTraceByChannel (Transformation|GetActorLocation) (* (Math|Vector|GetUpVector (Variables|Default|GetMeshroom)) -1e+08) "TraceTypeQuery4" false 0 "Persistent"))
      (Transformation|SetActorLocation (.location _outhit) true true))))

(fn ConstructionScript
  (bind _meshrooms (LocalVariables|GetMeshrooms))
  (bind (_outitem _outindex) (Utilities|Array|Random _meshrooms))
  (Variables|Default|SetMeshroomIndex _outindex)
  (if (Variables|Default|GetbSpawnedFromMushroom)
    _
    (else
      (Components|StaticMesh|SetStaticMesh (Variables|Default|GetMeshroom) _outitem)))
  (|CallParentFunction))