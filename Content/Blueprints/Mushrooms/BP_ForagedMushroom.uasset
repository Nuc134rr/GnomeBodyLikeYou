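; Foraged mushroom actor that randomly becomes a rare variant, with its item data and mesh taken from the foragable data table.
; The construction script rolls 0 to 100 against nested thresholds for gold, bronze or silver, and glowing rows, deferring to the parent script on higher rolls.
; The checks run in sequence without exclusion, so a found glowing row overwrites any gold, bronze or silver pick.
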(event EventBeginPlay
  (|CallParentFunction))

(event Collision|EventActorBeginOverlap
  (params (OtherActor :type Actor%20Object%20Reference)))

(event EventTick
  (params (DeltaSeconds :type Float%20%28single-precision%29))
  (|CallParentFunction DeltaSeconds))

(fn ConstructionScript
  (bind _meshroom (Variables|Default|GetMeshroom))
  (LocalVariables|SetRandomValue (Math|Random|RandomIntegerinRange 0 100))
  (Utilities|FlowControl|Sequence
    (:then_0
      (if (<= (LocalVariables|GetRandomValue) 2)
        (bind _returnvalue (Utilities|GetDataTableRow "/Game/Blueprints/Core/Inventory/ForagableDataTable.ForagableDataTable" "GoldMushroom")
          (:then
            (bind _output_get (Variables|/Game/Blueprints/Core/Inventory/ItemDataComponent.ItemDataComponent_C|SetItemID (Variables|Default|GetItemDataComponent) _returnvalue))
            (Components|StaticMesh|SetStaticMesh _meshroom (.mushroommesh _output_get))))))
    (:then_1
      (if (<= (LocalVariables|GetRandomValue) 5)
        (bind _returnvalue_2 (Utilities|GetDataTableRow "/Game/Blueprints/Core/Inventory/ForagableDataTable.ForagableDataTable" (select (Math|Random|RandomBool) "BronzeMushroom" "SilverMushroom"))
          (:then
            (bind _output_get_2 (Variables|/Game/Blueprints/Core/Inventory/ItemDataComponent.ItemDataComponent_C|SetItemID (Variables|Default|GetItemDataComponent) _returnvalue_2))
            (Components|StaticMesh|SetStaticMesh _meshroom (.mushroommesh _output_get_2))))))
    (:then_2
      (if (<= (LocalVariables|GetRandomValue) 10)
        (bind _returnvalue_3 (Utilities|GetDataTableRow "/Game/Blueprints/Core/Inventory/ForagableDataTable.ForagableDataTable" "GlowingMushroom")
          (:then
            (bind _output_get_3 (Variables|/Game/Blueprints/Core/Inventory/ItemDataComponent.ItemDataComponent_C|SetItemID (Variables|Default|GetItemDataComponent) _returnvalue_3))
            (Components|StaticMesh|SetStaticMesh _meshroom (.mushroommesh _output_get_3))))
        (else
          (|CallParentFunction))))))